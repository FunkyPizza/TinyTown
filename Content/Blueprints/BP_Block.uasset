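; BP_Block is a grid block actor that shows a building, zone or road according to its BlockStats.
; On BeginPlay it scales the base cube and building from the stats and tints buildings by grid colour; zones get random snapped heights, while paths become flat charcoal slabs.
; A valid stats mesh instead swaps in a placeholder editor sphere.
; A Delay-throttled Tick feeds TT_GameState hours and minutes into the building materials.
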(event `self.ReceiveBeginPlay`
  (bind (_blockstats_block_name _blockstats_description _blockstats_category_name _blockstats_block_type _blockstats_resizable _blockstats_size_x _blockstats_size_y _blockstats_grid_colour _blockstats_efficiency _blockstats_initial_cost _blockstats_r_mo _blockstats_r_po _blockstats_r_ha _blockstats_r_el _blockstats_r_wa _blockstats_r_in _blockstats_r_pr _blockstats_p_mo _blockstats_p_po _blockstats_p_ha _blockstats_p_el _blockstats_p_wa _blockstats_p_in _blockstats_p_pr _blockstats_mesh) (break `TT_Struct_Block` (`self.blockStats`)))
  (bind _returnvalue (* _blockstats_size_y 2.5))
  (bind _returnvalue_2 (* _blockstats_size_x 2.5))
  (`/Engine/EditorBlueprintResources/StandardMacros.IsValid` _blockstats_mesh
    (:`Is Valid`
      (`StaticMeshComponent.SetStaticMesh` (`self.Building`) "/Engine/EditorMeshes/ArcadeEditorSphere.ArcadeEditorSphere"))
    (:`Is Not Valid`
      (`SceneComponent.SetRelativeScale3D` (`self.Cube`) (`KismetMathLibrary.MakeVector` _returnvalue_2 _returnvalue (select `bool` (`|EnumEquality` _blockstats_block_type "BT_Path") :`false` 0.3 :`true` 0.1 :!type "Float (single-precision)")))
      (switch `EBlockType` _blockstats_block_type
        (:`BT_Building`
          ;[0 0 0] Block is a building
          (`SceneComponent.SetRelativeScale3D` (`self.Building`) (`KismetMathLibrary.MakeVector` (* _returnvalue_2 0.8) (* _returnvalue 0.8) 6.0))
          (`MeshComponent.SetVectorParameterValueOnMaterials` (`self.Building`) "BuildingColour" (`KismetMathLibrary.Conv_LinearColorToVector` _blockstats_grid_colour)))
        (:`BT_ZoneBuilding`
          ;[0 0 0] Block is a building
          (`SceneComponent.SetRelativeScale3D` (`self.Building`) (`KismetMathLibrary.MakeVector` (* _returnvalue_2 0.8) (* _returnvalue 0.8) (`KismetMathLibrary.GridSnap_Float` (`KismetMathLibrary.RandomFloatInRange` 3.0 6.0) 1.0)) :!label _label)
          (`MeshComponent.SetVectorParameterValueOnMaterials` (`self.Building`) "BuildingColour" (`KismetMathLibrary.Conv_LinearColorToVector` _blockstats_grid_colour)))
        (:`BT_Zone`
          (goto _label))
        (:`BT_Path`
          ;[0 0 0] Block is a road
          (`ActorComponent.K2_DestroyComponent` (`self.Building`))
          (`PrimitiveComponent.SetMaterial` (`self.Cube`) 0 "/Game/Assets/Materials/M_CharcoalLight.M_CharcoalLight"))))))

(event `self.ReceiveTick`
  (params (DeltaSeconds :type "Float (single-precision)"))
  (bind _building (`self.Building`))
  (bind _astt_game_state (cast `TT_GameState` (`GameplayStatics.GetGameState`) :!pure true))
  (`KismetSystemLibrary.Delay` 0.2)
  (`/Engine/EditorBlueprintResources/StandardMacros.IsValid` _building
    (:`Is Valid`
      (`MeshComponent.SetScalarParameterValueOnMaterials` _building "Time" (`KismetMathLibrary.Conv_IntToDouble` (`TT_GameState.Time_Hours` _astt_game_state)))
      (`MeshComponent.SetScalarParameterValueOnMaterials` _building "Minutes" (`KismetMathLibrary.Conv_IntToDouble` (`TT_GameState.Time_Minutes` _astt_game_state))))))

(fn `UserConstructionScript`)