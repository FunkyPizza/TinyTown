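; Generic grid block actor that sizes and colours itself on BeginPlay from its block data.
; The cube and box collision scale to the footprint, with paths thinner than other types.
; Buildings get an inset, fixed-height mesh, while Zones and Zone Buildings get a random whole-number height scale.
; These types also take the grid colour as a material parameter and call ConstructionEffect according to editing mode.
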(event `self.ReceiveBeginPlay`
  (bind (_returnvalue_block_name _returnvalue_description _returnvalue_category_name _returnvalue_size_x _returnvalue_size_y _returnvalue_block_type _returnvalue_icon _returnvalue_blockclass _returnvalue_grid_colour) (break `TT_Struct_Block` (`self.GetBlockData`)))
  (bind _returnvalue (* _returnvalue_size_y 2.5))
  (bind _returnvalue_2 (* _returnvalue_size_x 2.5))
  ;[0.1979 0.1979 0.1979] Begin Play
  (`SceneComponent.SetRelativeScale3D` (`self.Cube`) (`KismetMathLibrary.MakeVector` _returnvalue_2 _returnvalue (select `bool` (`|EnumEquality` _returnvalue_block_type "BT_Path") :`false` 0.3 :`true` 0.1 :!type "Float (single-precision)")))
  (`SceneComponent.SetRelativeScale3D` (`self.BoxComp`) (`KismetMathLibrary.MakeVector` _returnvalue_2 _returnvalue (select `bool` (`|EnumEquality` _returnvalue_block_type "BT_Path") :`false` 0.3 :`true` 0.1 :!type "Float (single-precision)")))
  (switch `EBlockType` _returnvalue_block_type
    (:`BT_Building`
      ;;[0 0 0] Block is a building, set Z scale to 6, set the building color to the color set in data table.
      (`SceneComponent.SetRelativeScale3D` (`self.BlockMesh`) (`KismetMathLibrary.MakeVector` (* _returnvalue_2 0.8) (* _returnvalue 0.8) 6.0))
      (`SceneComponent.SetRelativeScale3D` (`self.BoxComp`) (`KismetMathLibrary.MakeVector` (* _returnvalue_2 0.8) (* _returnvalue 0.8) 6.0))
      (`MeshComponent.SetVectorParameterValueOnMaterials` (`self.BlockMesh`) "BuildingColour" (`KismetMathLibrary.Conv_LinearColorToVector` _returnvalue_grid_colour)))
    (:`BT_ZoneBuilding`
      ;;[0 0 0] Block is a building, set random Z scale, set the building color to the color set in data table.
      (`SceneComponent.SetRelativeScale3D` (`self.BlockMesh`) (`KismetMathLibrary.MakeVector` (* _returnvalue_2 0.8) (* _returnvalue 0.8) (`KismetMathLibrary.GridSnap_Float` (`KismetMathLibrary.RandomFloatInRange` 3.0 6.0) 1.0)) :!label _label)
      (`SceneComponent.SetRelativeScale3D` (`self.BoxComp`) (`KismetMathLibrary.MakeVector` (* _returnvalue_2 0.8) (* _returnvalue 0.8) (`KismetMathLibrary.GridSnap_Float` (`KismetMathLibrary.RandomFloatInRange` 3.0 6.0) 1.0)))
      (`MeshComponent.SetVectorParameterValueOnMaterials` (`self.BlockMesh`) "BuildingColour" (`KismetMathLibrary.Conv_LinearColorToVector` _returnvalue_grid_colour)))
    (:`BT_Zone`
      (goto _label)))
  (if (`self.isInEditingMode`)
    (`self.ConstructionEffect` true)
    (else
      (`self.ConstructionEffect` false))))

(fn `UserConstructionScript`)