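; Grid block actor that sizes and colours itself from its block data, covering paths, buildings and zones.
; BeginPlay scales mesh and collision by grid size and type, with fixed height for buildings and random snapped height for zones and zone buildings.
; Those types get a material-driven construction effect, animated by timeline or immediate in editing mode.
; Tick uses a 0.2-second delay to throttle feeding game-state time into the material.
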(event `self.OnDestroyBlock`
  ;[0.1979 0.1979 0.1979] TT_Block
  (`parent.OnDestroyBlock`))

(event `self.ReceiveBeginPlay`
  (bind (_returnvalue_block_name _returnvalue_description _returnvalue_category_name _returnvalue_block_type _returnvalue_size_x _returnvalue_size_y _returnvalue_grid_colour) (break `TT_Struct_Block` (`self.GetBlockData`)))
  (bind _returnvalue (* _returnvalue_size_y 2.5))
  (bind _returnvalue_2 (* _returnvalue_size_x 2.5))
  ;[0.1979 0.1979 0.1979] Begin Play
  (`SceneComponent.SetRelativeScale3D` (`self.Cube`) (`KismetMathLibrary.MakeVector` _returnvalue_2 _returnvalue (select `bool` (`|EnumEquality` _returnvalue_block_type "BT_Path") :`false` 0.3 :`true` 0.1 :!type "Float (single-precision)")))
  (`SceneComponent.SetRelativeScale3D` (`self.BoxComp`) (`KismetMathLibrary.MakeVector` _returnvalue_2 _returnvalue (select `bool` (`|EnumEquality` _returnvalue_block_type "BT_Path") :`false` 0.3 :`true` 0.1 :!type "Float (single-precision)")))
  (switch `EBlockType` _returnvalue_block_type
    (:`BT_Building`
      ;;[0 0 0] Block is a building, set Z scale to 6, set the building color to the color set in data table.
      (`SceneComponent.SetRelativeScale3D` (`self.BlockMesh`) (`KismetMathLibrary.MakeVector` (* _returnvalue_2 0.8) (* _returnvalue 0.8) 6.0))
      (`SceneComponent.SetRelativeScale3D` (`self.BoxComp`) (`KismetMathLibrary.MakeVector` (* _returnvalue_2 0.8) (* _returnvalue 0.8) 6.0))
      (`MeshComponent.SetVectorParameterValueOnMaterials` (`self.BlockMesh`) "BuildingColour" (`KismetMathLibrary.Conv_LinearColorToVector` _returnvalue_grid_colour)))
    (:`BT_ZoneBuilding`
      ;;[0 0 0] Block is a building, set random Z scale, set the building color to the color set in data table.
      (`SceneComponent.SetRelativeScale3D` (`self.BlockMesh`) (`KismetMathLibrary.MakeVector` (* _returnvalue_2 0.8) (* _returnvalue 0.8) (`KismetMathLibrary.GridSnap_Float` (`KismetMathLibrary.RandomFloatInRange` 3.0 6.0) 1.0)) :!label _label)
      (`SceneComponent.SetRelativeScale3D` (`self.BoxComp`) (`KismetMathLibrary.MakeVector` (* _returnvalue_2 0.8) (* _returnvalue 0.8) (`KismetMathLibrary.GridSnap_Float` (`KismetMathLibrary.RandomFloatInRange` 3.0 6.0) 1.0)))
      (`MeshComponent.SetVectorParameterValueOnMaterials` (`self.BlockMesh`) "BuildingColour" (`KismetMathLibrary.Conv_LinearColorToVector` _returnvalue_grid_colour)))
    (:`BT_Zone`
      (goto _label)))
  (if (`self.isInEditingMode`)
    (`self.ConstructionEffect` true)
    (else
      (`self.ConstructionEffect` false))))

(event `ConstructionEffect`
  (params (isImmediate :type Boolean))
  (bind _blockmesh (`self.BlockMesh`))
  (bind _blockmesh_2 (`self.BlockMesh`))
  (bind (_relativescale3d_x _relativescale3d_y _relativescale3d_z) (`KismetMathLibrary.BreakVector` (`SceneComponent.RelativeScale3D` _blockmesh)))
  (bind (_relativescale3d_x_2 _relativescale3d_y_2 _relativescale3d_z_2) (`KismetMathLibrary.BreakVector` (`SceneComponent.RelativeScale3D` _blockmesh_2)))
  ;[0.1979 0.1979 0.1979] Construction material set up ("Construction" effect that happens when a block is spawned).
  (if isImmediate
    (`MeshComponent.SetScalarParameterValueOnMaterials` (`self.BlockMesh`) "BuildingHeight" (* (.z (`.Max` (`StaticMeshComponent.GetLocalBounds` _blockmesh))) _relativescale3d_z))
    (`MeshComponent.SetScalarParameterValueOnMaterials` (`self.BlockMesh`) "ConstructionAlpha" 1.1)
    (else
      (`MeshComponent.SetScalarParameterValueOnMaterials` (`self.BlockMesh`) "BuildingHeight" (* (.z (`.Max` (`StaticMeshComponent.GetLocalBounds` _blockmesh_2))) _relativescale3d_z_2))
      (bind (_direction _alpha) (`Timeline|Timeline_BlockScaleUp` :!via `PlayFromStart`)
        (:`Update`
          (`MeshComponent.SetScalarParameterValueOnMaterials` (`self.BlockMesh`) "ConstructionAlpha" _alpha))))))

(event `self.ReceiveTick`
  (params (DeltaSeconds :type "Float (single-precision)"))
  (bind _blockmesh (`self.BlockMesh`))
  (bind _astt_game_state (cast `TT_GameState` (`GameplayStatics.GetGameState`) :!pure true))
  ;[0.1979 0.1979 0.1979] Event Tick
  ;;[0 0 0] Update the block's material
  (`KismetSystemLibrary.Delay` 0.2)
  (`/Engine/EditorBlueprintResources/StandardMacros.IsValid` _blockmesh
    (:`Is Valid`
      (`MeshComponent.SetScalarParameterValueOnMaterials` _blockmesh "Time" (`KismetMathLibrary.Conv_IntToDouble` (`TT_GameState.Time_Hours` _astt_game_state)))
      (`MeshComponent.SetScalarParameterValueOnMaterials` _blockmesh "Minutes" (`KismetMathLibrary.Conv_IntToDouble` (`TT_GameState.Time_Minutes` _astt_game_state))))))

(fn `UserConstructionScript`)