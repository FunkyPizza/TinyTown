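; BP_BlockParent is a base block actor that drives its mesh materials for a construction effect and time of day.
; On BeginPlay it sets the building height from the mesh bounds and scale, then animates ConstructionAlpha with a timeline, or sets it instantly in editing mode.
; Tick, through a short Delay, feeds the TT_GameState hours and minutes into the material's scalar parameters.
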(event `self.ReceiveBeginPlay`
  (if (`self.isInEditingMode`)
    (`self.ConstructionEffect` true)
    (else
      (`self.ConstructionEffect` false))))

(event `self.ReceiveTick`
  (params (DeltaSeconds :type "Float (single-precision)"))
  (bind _blockmesh (`self.BlockMesh`))
  (bind _astt_game_state (cast `TT_GameState` (`GameplayStatics.GetGameState`) :!pure true))
  ;[0.1979 0.1979 0.1979] Event Tick
  ;;[0 0 0] Update the block's material
  (`KismetSystemLibrary.Delay` 0.2)
  (`/Engine/EditorBlueprintResources/StandardMacros.IsValid` _blockmesh
    (:`Is Valid`
      (`MeshComponent.SetScalarParameterValueOnMaterials` _blockmesh "Time" (`KismetMathLibrary.Conv_IntToDouble` (`TT_GameState.Time_Hours` _astt_game_state)))
      (`MeshComponent.SetScalarParameterValueOnMaterials` _blockmesh "Minutes" (`KismetMathLibrary.Conv_IntToDouble` (`TT_GameState.Time_Minutes` _astt_game_state))))))

(event `ConstructionEffect`
  (params (isImmediate :type Boolean))
  (bind _blockmesh (`self.BlockMesh`))
  (bind _blockmesh_2 (`self.BlockMesh`))
  (bind (_relativescale3d_x _relativescale3d_y _relativescale3d_z) (`KismetMathLibrary.BreakVector` (`SceneComponent.RelativeScale3D` _blockmesh)))
  (bind (_relativescale3d_x_2 _relativescale3d_y_2 _relativescale3d_z_2) (`KismetMathLibrary.BreakVector` (`SceneComponent.RelativeScale3D` _blockmesh_2)))
  ;[0.1979 0.1979 0.1979] Construction material set up ("Construction" effect that happens when a block is spawned).
  (if isImmediate
    (`MeshComponent.SetScalarParameterValueOnMaterials` (`self.BlockMesh`) "BuildingHeight" (* (.z (`.Max` (`StaticMeshComponent.GetLocalBounds` _blockmesh))) _relativescale3d_z))
    (`MeshComponent.SetScalarParameterValueOnMaterials` (`self.BlockMesh`) "ConstructionAlpha" 1.1)
    (else
      (`MeshComponent.SetScalarParameterValueOnMaterials` (`self.BlockMesh`) "BuildingHeight" (* (.z (`.Max` (`StaticMeshComponent.GetLocalBounds` _blockmesh_2))) _relativescale3d_z_2))
      (bind (_direction _alpha) (`Timeline|Timeline_0` :!via `PlayFromStart`)
        (:`Update`
          (`MeshComponent.SetScalarParameterValueOnMaterials` (`self.BlockMesh`) "ConstructionAlpha" _alpha))))))

(fn `UserConstructionScript`)