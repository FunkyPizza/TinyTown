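; Player grid camera Blueprint that handles input for moving, rotating and zooming the view, selecting, cancelling and removing blocks.
; On BeginPlay it creates the W_UI widget, adds it to the viewport and passes itself as its Player.
; Keyboard and mouse events only forward to input functions defined outside these graphs.
; Both movement axes share one InputKeyboardMovements call with a constant zero rather than their axis values.
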(event `self.ReceiveBeginPlay`
  (bind _returnvalue (`|CreateWidget` "/Game/Blueprints/UI/W_UI.W_UI_C"))
  (`UserWidget.AddToViewport` _returnvalue 0)
  (set `/Game/Blueprints/UI/W_UI.Player` self _returnvalue))

(event `InputAxis|XRotation` :consume false
  (params (AxisValue :type "Float (single-precision)"))
  ;[0.1979 0.1979 0.1979] Controls
  ;;[0 0 0] Keyboard
  (`self.InputKeyboardRotation` AxisValue))

(event `InputAction|Delete`
  (params (Key :type "Key Structure"))
  ;[0.1979 0.1979 0.1979] Controls
  ;;[0 0 0] Keyboard
  (:`Pressed`
    (`self.RemoveBlockUnderCursor`)))

(event `InputAxis|MoveForward`
  (params (AxisValue :type "Float (single-precision)"))
  ;[0.1979 0.1979 0.1979] Controls
  ;;[0 0 0] Keyboard
  (`self.InputKeyboardMovements` 0.0 :!label _label))

(event `self.ReceiveTick`
  (params (DeltaSeconds :type "Float (single-precision)")))

(event `InputAxis|MoveRight`
  (params (AxisValue :type "Float (single-precision)"))
  ;[0.1979 0.1979 0.1979] Controls
  ;;[0 0 0] Keyboard
  (goto _label))

(event `InputAction|InputMovement` :consume false
  (params (Key :type "Key Structure"))
  ;[0.1979 0.1979 0.1979] Controls
  ;;[0 0 0] Mouse
  (:`Pressed`
    (`self.InputMoveButtonDown`))
  (:`Released`
    (`self.InputMoveButtonUp`)))

(event `InputAction|InputSelect` :consume false
  (params (Key :type "Key Structure"))
  ;[0.1979 0.1979 0.1979] Controls
  ;;[0 0 0] Mouse
  (:`Pressed`
    (`self.InputSelectButtonDown`))
  (:`Released`
    (`self.InputSelectButtonUp`)))

(event `InputAction|InputRotation` :consume false
  (params (Key :type "Key Structure"))
  ;[0.1979 0.1979 0.1979] Controls
  ;;[0 0 0] Mouse
  (:`Pressed`
    (`self.InputRotationButtonDown`))
  (:`Released`
    (`self.InputRotationButtonUp`)))

(event `InputAction|InputCancel` :consume false
  (params (Key :type "Key Structure"))
  ;[0.1979 0.1979 0.1979] Controls
  ;;[0 0 0] Mouse
  (:`Released`
    (`self.InputCancel`)))

(event `InputAxis|ZoomIn` :consume false
  (params (AxisValue :type "Float (single-precision)"))
  ;[0.1979 0.1979 0.1979] Controls
  ;;[0 0 0] Mouse
  (`self.InputCameraZoom` AxisValue))

(fn `UserConstructionScript`)