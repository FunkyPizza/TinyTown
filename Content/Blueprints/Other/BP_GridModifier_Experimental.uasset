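; Experimental grid-editing tool that shifts BP_GridManager tiles inside its box by DesiredOffset.
; The construction script box-traces on Visibility and uses each hit item as a tile ID, offsetting tiles not already in ModifiedTiles.
; It then subtracts the offset for tracked tiles outside the box, but omits their TileID and never untracks them.
; ResetTool reverses offsets and clears tracking, though it writes by array index rather than stored tile ID.
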(event `ResetTool`
  ;[0.1979 0.1979 0.1979] Reset affected tiles
  (bind (_arrayindex _arrayelement) (`/Engine/EditorBlueprintResources/StandardMacros.ReverseForEachLoop` (`self.ModifiedTiles`))
    (:`LoopBody`
      (`TT_GridManager.SetTileTransform` (`self.GridManager`) _arrayindex (`KismetMathLibrary.MakeTransform` (- (`TT_GridManager.GetTileLocation` (`self.GridManager`) _arrayelement false) (`self.DesiredOffset`))) false))
    (:`Completed`
      (`KismetArrayLibrary.Array_Clear` (`self.OverlappingTiles`))
      (`KismetArrayLibrary.Array_Clear` (`self.ModifiedTiles`)))))

(fn `UserConstructionScript`
  (bind _box (`self.Box`))
  (bind _returnvalue (`SceneComponent.K2_GetComponentLocation` _box))
  ;[0.1979 0.1979 0.1979] Get collisions in box radius. (The Box component is only for visual aspect)
  (bind (_outhits _returnvalue_2) (`KismetSystemLibrary.BoxTraceMulti` :`Start` _returnvalue :`End` (+ _returnvalue (1.0 0.0 0.0)) :`HalfSize` (`BoxComponent.GetScaledBoxExtent` _box) :`TraceChannel` "TraceTypeQuery1" :`bTraceComplex` true :`bIgnoreSelf` false :`DrawTime` 1.0))
  (if _returnvalue_2
    (for _array_element _outhits
      ;[0.1979 0.1979 0.1979] Offset all the colliding tiles
      (bind _asbp_grid_manager (cast `/Game/Blueprints/BP_GridManager` (`.HitActor` (`GameplayStatics.BreakHitResult` _array_element))))
      (`|ExecutionSequence`
        (:`then_0`
          (`/Engine/EditorBlueprintResources/StandardMacros.DoOnce` false
            (:`Completed`
              (set `self.GridManager` _asbp_grid_manager))))
        (:`then_1`
          (`KismetArrayLibrary.Array_Add` (`self.OverlappingTiles`) (`.HitItem` (`GameplayStatics.BreakHitResult` _array_element)))
          (if (not (`KismetArrayLibrary.Array_Contains` (`self.ModifiedTiles`) (`.HitItem` (`GameplayStatics.BreakHitResult` _array_element))))
            (`TT_GridManager.SetTileTransform` _asbp_grid_manager (`.HitItem` (`GameplayStatics.BreakHitResult` _array_element)) (`KismetMathLibrary.MakeTransform` (+ (`TT_GridManager.GetTileLocation` _asbp_grid_manager (`.HitItem` (`GameplayStatics.BreakHitResult` _array_element)) false) (`self.DesiredOffset`))) false)
            (`KismetArrayLibrary.Array_Add` (`self.ModifiedTiles`) (`.HitItem` (`GameplayStatics.BreakHitResult` _array_element)))))))
    ;[0.1979 0.1979 0.1979] Reset all modified tiles that aren't colliding anymore
    (bind (_arrayindex _arrayelement) (`/Engine/EditorBlueprintResources/StandardMacros.ReverseForEachLoop` (`self.ModifiedTiles`))
      (:`LoopBody`
        (if (not (`KismetArrayLibrary.Array_Contains` (`self.OverlappingTiles`) _arrayelement))
          (`TT_GridManager.SetTileTransform` (`self.GridManager`) 0 (`KismetMathLibrary.MakeTransform` (- (`TT_GridManager.GetTileLocation` (`self.GridManager`) _arrayelement false) (`self.DesiredOffset`))) false)))
      (:`Completed`
        (`KismetArrayLibrary.Array_Clear` (`self.OverlappingTiles`))))))